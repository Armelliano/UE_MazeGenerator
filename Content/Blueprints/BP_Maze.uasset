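; Procedural maze actor that builds a seeded tile maze in its construction script, placing Hierarchical Instanced Static Mesh instances on a TileSize grid.
; GenerateMaze runs randomized depth-first search from a random start: AddNeighbourLoc recursively carves cells two steps apart, recording the bridge tile between them.
; When stuck, BackTrack pops the latest cell and moves its bridge into the path.
; Dead ends are collected and returned, but only path tiles are rendered.
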(fn `AddNeighbourLoc`
  (params (Size :type "IntPoint Structure (by ref)") (RandStream :type "RandomStream Structure (by ref)") (CurrentLoc :type "IntPoint Structure (by ref)") (PathTiles :type "Set of IntPoint Structure (by ref)") (BridgeTiles :type "Set of IntPoint Structure (by ref)") (ToCheck :type "Set of IntPoint Structure (by ref)") (EndPaths :type "Set of IntPoint Structure (by ref)"))
  (locals (NeighbourIndex :type Integer))
  (bind (_floor _bridge) (`self.GetNeighbourAndBridge` (`local.CurrentLoc`) (`local.NeighbourIndex`)))
  (bind _returnvalue (+ (`local.NeighbourIndex`) 1))
  (set `local.NeighbourIndex` (`KismetMathLibrary.RandomIntegerInRangeFromStream` (`local.RandStream`) 0 3))
  (if (`self.CheckIsValidLoc` (`self.GetNeighbourAndBridge` (`local.CurrentLoc`) (`local.NeighbourIndex`)) (`local.Size`) (`local.PathTiles`) (`local.BridgeTiles`)) :!label _label
    ;[1 1 1] If true, set the current tile as a possible path or bridge tile and save it
    (`BlueprintSetLibrary.Set_Add` (`local.PathTiles`) _floor)
    (`BlueprintSetLibrary.Set_Add` (`local.BridgeTiles`) _bridge)
    (`BlueprintSetLibrary.Set_Add` (`local.ToCheck`) _floor)
    (`self.AddNeighbourLoc` (`local.Size`) (`local.RandStream`) _floor (`local.PathTiles`) (`local.BridgeTiles`) (`local.ToCheck`) (`local.EndPaths`))
    (else
      ;[1 1 1] Else, if NeighbourIndex value equal 4, set NeighbourIndex value to 0, elsewhere increase it by 1, than re-check tile with new value
      (`/Game/Blueprints/CustomMacLib.DoN+` 4
        (:`Exit`
          (set `local.NeighbourIndex` (`KismetMathLibrary.SelectInt` 0 _returnvalue (> _returnvalue 3)))
          (goto _label))
        (:`OverNth`
          ;[1 1 1] If it's a end-path tile, save it to end-path tile list
          (bind _count (`self.Get Neighbour Count` (`local.CurrentLoc`) (`local.PathTiles`)))
          (if (== _count 1)
            (`BlueprintSetLibrary.Set_Add` (`local.EndPaths`) (`local.CurrentLoc`))))))))

(fn `BackTrack`
  (params (CurrentTIle :type "IntPoint Structure (by ref)") (ToCheck :type "Set of IntPoint Structure (by ref)") (BridgeTIles :type "Set of IntPoint Structure (by ref)") (PathTiles :type "Set of IntPoint Structure (by ref)"))
  ;[1 1 1] Clear the list of tiles from in reverse order (from last to first)
  (bind _result (`BlueprintSetLibrary.Set_ToArray` ToCheck))
  (bind _output (`|GetArrayItem` _result (`KismetArrayLibrary.Array_LastIndex` _result)))
  (`|VariableSetRef` (`local.CurrentTIle`) _output)
  (`BlueprintSetLibrary.Set_Remove` (`local.ToCheck`) _output)
  (bind _result_2 (`BlueprintSetLibrary.Set_ToArray` (`local.BridgeTIles`)))
  (bind _output_2 (`|GetArrayItem` _result_2 (`KismetArrayLibrary.Array_LastIndex` _result_2)))
  (`BlueprintSetLibrary.Set_Add` (`local.PathTiles`) _output_2)
  (`BlueprintSetLibrary.Set_Remove` (`local.BridgeTIles`) _output_2))

(fn `GenerateMaze`
  (params (Seed :type Integer) (Size :type "IntPoint Structure"))
  (returns (PathTiles_Out :type "Set of IntPoint Structure") (EndPath_Out :type "Set of IntPoint Structure"))
  (locals (RandStream :type "RandomStream Structure") (L_Size :type "IntPoint Structure") (StartingLoc :type "IntPoint Structure") (CurrentLoc :type "IntPoint Structure") (PathTiles :type "Set of IntPoint Structure") (BridgeTiles :type "Set of IntPoint Structure") (ToCheck :type "Set of IntPoint Structure") (EndPaths :type "Set of IntPoint Structure"))
  (`KismetMathLibrary.SetRandomStreamSeed` (`local.RandStream`) Seed)
  (set `local.L_Size` Size) ; Know the lenght size
  (bind _output_get (set `local.StartingLoc` (`self.GetRandLocInBounds` (`local.L_Size`) (`local.RandStream`)))) ; Set random position as start position
  (set `local.CurrentLoc` _output_get) ; Set current position equal to start position
  ;[1 1 1] Repeat control until there left no tiles to check
  (`self.AddNeighbourLoc` (`local.L_Size`) (`local.RandStream`) (`local.CurrentLoc`) (`local.PathTiles`) (`local.BridgeTiles`) (`local.ToCheck`) (`local.EndPaths`) :!label _label) ; Check next neighbour tile
  ;;[1 1 1] If there are tiles to check (>0) return the tile, elsewhere return the list of valid path tiles and end-path tile
  (if (> (`BlueprintSetLibrary.Set_Length` (`local.ToCheck`)) 0)
    (`self.BackTrack` (`local.CurrentLoc`) (`local.ToCheck`) (`local.BridgeTiles`) (`local.PathTiles`))
    (goto _label)
    (else
      (return (`local.PathTiles`) (`local.EndPaths`)))))

(fn `Get Neighbour Count`
  (params (CurrentLoc :type "IntPoint Structure (by ref)") (PathTiles :type "Set of IntPoint Structure (by ref)"))
  (returns (Count :type Integer))
  (locals (Counter :type Integer))
  ;[1 1 1] Check if target tiles is the end of the path and return the value of neighbour tiles already in use
  (for _array_element (`self.GetNeighbourLoc` CurrentLoc 1)
    (if (`BlueprintSetLibrary.Set_Contains` (`local.PathTiles`) _array_element)
      (`/Engine/EditorBlueprintResources/StandardMacros.IncrementInt` (`local.Counter`)
        (:`  `
          (`KismetSystemLibrary.PrintString` "Hello")))))
  (return (`local.Counter`)))

(fn `UserConstructionScript`
  (bind _tilesize (`self.TileSize`))
  ;[1 1 1] Populate maze with tile's mesh
  (bind _pathtiles_out (`self.GenerateMaze` (`self.Seed`) (`self.Size`)))
  (bind _result (`BlueprintSetLibrary.Set_ToArray` _pathtiles_out))
  ;;[1 1 1] Place the next maze tile next to the previous one, considering size
  (for _array_element _result
    (bind (_x _y) (break `IntPoint` _array_element))
    (`InstancedStaticMeshComponent.AddInstance` (`self.HierarchicalInstancedStaticMesh`) (`KismetMathLibrary.MakeTransform` (`KismetMathLibrary.MakeVector` (* _x _tilesize) (* _y _tilesize))) true)))